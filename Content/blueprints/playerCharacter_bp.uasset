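; First-person player character Blueprint handling movement, mouse look, sprinting, crouching and double jumping.
; Forward and strafe axes move along a ForwardArrow that yaws with the mouse, while camera pitch is clamped and walk speed follows sprint and crouch flags.
; Crouch squashes actor Z scale.
; A downward line trace each Tick detects ground to manage sprint state and the jump count for LaunchCharacter jumps.
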(event EventBeginPlay
  (Variables|Default|Setsens 1.0)
  (Variables|/Script/Engine.CharacterMovementComponent|SetAirControl (Variables|Character|GetCharacterMovement) 1.0))

(event EventTick
  (params (DeltaSeconds :type Float%20%28single-precision%29))
  (bind _returnvalue (Transformation|GetActorLocation))
  (bind _returnvalue_2 (Collision|LineTraceForObjects _returnvalue (+ _returnvalue (Math|Vector|MakeVector 0.0 0.0 (- (- 0.0 (.OutHalfHeight (Components|Capsule|GetScaledCapsuleSize (Variables|Collision|GetCapsuleComponent)))) 22.0))) (Utilities|Array|MakeArray "ObjectTypeQuery2") false 0 "None"))
  (if _returnvalue_2
    (Variables|Default|SetjumpCount 1)
    (if (> (Class|PlayerController|GetInputKeyTimeDown (Game|GetPlayerController 0) (stale Input|ActionEvents|InputActionsprintKey Key)) 0.1)
      (Variables|Default|Setshift_pressed true))
    (else
      (Variables|Default|Setshift_pressed false)))
  (if (not (<= 0.3 (stale Input|AxisEvents|InputAxisForwardKey AxisValue)))
    (Variables|Default|Setshift_pressed false)))

(event Input|ActionEvents|InputActionsprintKey
  (params (Key :type Key%20Structure))
  (:Pressed
    (Variables|Default|Setshift_pressed true)))

(event Input|ActionEvents|InputActioncrouchKey
  (params (Key :type Key%20Structure))
  (:Pressed
    (Variables|Default|Setcrouch_pressed true)
    (Transformation|SetActorScale3D "1.000000,1.000000,0.500000")
    (Variables|Default|Setshift_pressed false))
  (:Released
    (Variables|Default|Setcrouch_pressed false)
    (Transformation|SetActorScale3D "1.000000,1.000000,1.000000")))

(event Input|ActionEvents|InputActionjumpKey
  (params (Key :type Key%20Structure))
  (:Pressed
    (Variables|Default|SetjumpLimit 2)
    (if (stale EventTick _returnvalue_2)
      (Variables|Default|SetjumpCount 1)
      (bind _output_get (Variables|Default|SetjumpPower 5e+02 :!label _label))
      (Character|LaunchCharacter self (* "0,0.000000,1.000000" _output_get) false false)
      (else
        (bind _output_get_2 (Variables|Default|SetjumpCount (+ (Variables|Default|GetjumpCount) 1)))
        (if (<= _output_get_2 2)
          (goto _label))))))

(event Input|AxisEvents|InputAxisForwardKey
  (params (AxisValue :type Float%20%28single-precision%29))
  (bind _charactermovement (Variables|Character|GetCharacterMovement))
  (if (Math|Boolean|ANDBoolean (> AxisValue 0.0) (Variables|Default|Getshift_pressed) (not (Variables|Default|Getcrouch_pressed)))
    (Variables|/Script/Engine.CharacterMovementComponent|SetMaxWalkSpeed (Variables|Character|GetCharacterMovement) 1e+03)
    (elif (Variables|Default|Getcrouch_pressed)
      (Variables|/Script/Engine.CharacterMovementComponent|SetMaxWalkSpeed _charactermovement 2.5e+02)
      (else
        (Variables|/Script/Engine.CharacterMovementComponent|SetMaxWalkSpeed _charactermovement 5e+02))))
  (Pawn|Input|AddMovementInput (* (Math|Vector|Normalize (+ (* (Math|Vector|GetRightVector (Variables|Default|GetforwardArrow)) (stale Input|AxisEvents|InputAxisstrafeKey AxisValue)) (* (Math|Vector|GetForwardVector (Variables|Default|GetforwardArrow)) AxisValue))) (Variables|/Script/Engine.CharacterMovementComponent|GetMaxWalkSpeed (Variables|Character|GetCharacterMovement))) 1.0 false))

(event Input|AxisEvents|InputAxisstrafeKey
  (params (AxisValue :type Float%20%28single-precision%29))
  (Pawn|Input|AddMovementInput (* (Math|Vector|Normalize (+ (* (Math|Vector|GetRightVector (Variables|Default|GetforwardArrow)) AxisValue) (* (Math|Vector|GetForwardVector (Variables|Default|GetforwardArrow)) (stale Input|AxisEvents|InputAxisForwardKey AxisValue)))) (Variables|/Script/Engine.CharacterMovementComponent|GetMaxWalkSpeed (Variables|Character|GetCharacterMovement))) 1.0 false))

(event Input|AxisEvents|InputAxisMouseX
  (params (AxisValue :type Float%20%28single-precision%29))
  (bind _playercamera (Variables|Default|GetplayerCamera))
  (bind _returnvalue (Transformation|GetWorldRotation _playercamera))
  (Transformation|AddRelativeRotation (Variables|Default|GetplayerCamera) (* (Math|Rotator|MakeRotator 0.0 (stale Input|AxisEvents|InputAxisMouseY AxisValue) AxisValue) (Variables|Default|Getsens)) false false)
  (Transformation|AddRelativeRotation (Variables|Default|GetforwardArrow) (Math|Rotator|MakeRotator 0.0 0.0 AxisValue) false false)
  (Transformation|SetWorldRotation _playercamera (Math|Rotator|MakeRotator 0.0 (Math|Float|ClampAngle (.pitch _returnvalue) -7e+01 7e+01) (.yaw _returnvalue)) false false))

(event Input|AxisEvents|InputAxisMouseY
  (params (AxisValue :type Float%20%28single-precision%29))
  (bind _playercamera (Variables|Default|GetplayerCamera))
  (bind _returnvalue (Transformation|GetWorldRotation _playercamera))
  (Transformation|AddRelativeRotation (Variables|Default|GetplayerCamera) (* (Math|Rotator|MakeRotator 0.0 AxisValue (stale Input|AxisEvents|InputAxisMouseX AxisValue)) (Variables|Default|Getsens)) false false)
  (Transformation|AddRelativeRotation (Variables|Default|GetforwardArrow) (Math|Rotator|MakeRotator 0.0 0.0 (stale Input|AxisEvents|InputAxisMouseX AxisValue)) false false)
  (Transformation|SetWorldRotation _playercamera (Math|Rotator|MakeRotator 0.0 (Math|Float|ClampAngle (.pitch _returnvalue) -7e+01 7e+01) (.yaw _returnvalue)) false false))

(fn ConstructionScript)